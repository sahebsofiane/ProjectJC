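; BP_BuildingCore is a building core actor that moves vertically until it is touched, then counts as destroyed.
; On BeginPlay a slowed timeline adds a Z offset to the static mesh's starting world location, without sweeping.
; Any component overlap or hit on the mesh enables gravity, stops the timeline and calls the EVDestroyedCore dispatcher, with no filter or one-shot guard.
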(event OnComponentBeginOverlap(StaticMeshComponent)
  (params (OverlappedComponent :type Primitive%20Component%20Object%20Reference) (OtherActor :type Actor%20Object%20Reference) (OtherComp :type Primitive%20Component%20Object%20Reference) (OtherBodyIndex :type Integer) (bFromSweep :type Boolean) (SweepResult :type Hit%20Result%20Structure%20%28by%20ref%29))
  (Physics|SetEnableGravity (Variables|Debug|GetStaticMeshComponent) true)
  (Audio|Components|Audio|Stop (Variables|Default|GetTimeline_0))
  (Default|CallEVDestroyedCore))

(event OnComponentHit(StaticMeshComponent)
  (params (HitComponent :type Primitive%20Component%20Object%20Reference) (OtherActor :type Actor%20Object%20Reference) (OtherComp :type Primitive%20Component%20Object%20Reference) (NormalImpulse :type Vector :default "0, 0, 0") (Hit :type Hit%20Result%20Structure%20%28by%20ref%29))
  (Physics|SetEnableGravity (Variables|Debug|GetStaticMeshComponent) true)
  (Audio|Components|Audio|Stop (Variables|Default|GetTimeline_0))
  (Default|CallEVDestroyedCore))

(event EventBeginPlay
  (Variables|Default|SetLocationa (Transformation|GetWorldLocation (Variables|Debug|GetStaticMeshComponent)))
  (Components|Timeline|SetPlayRate (Variables|Default|GetTimeline_0) 0.1)
  (bind _newtrack_0 (Timeline|Timeline_0 PlayFromStart)
    (:Update
      (Transformation|SetWorldLocation (Variables|Debug|GetStaticMeshComponent) (+ (Variables|Default|GetLocationa) (Math|Vector|MakeVector 0.0 0.0 _newtrack_0)) false false))))

(event Collision|EventActorBeginOverlap
  (params (OtherActor :type Actor%20Object%20Reference)))

(event EventTick
  (params (DeltaSeconds :type Float%20%28single-precision%29)))

(fn ConstructionScript)