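; End-of-demo zone that collects the Blue, Yellow and Red dancers, then lets the player finish the demo.
; The capsule overlap ejects each dancer's pawn and lights its spotlight; a MultiGate sets IsWinnable on the third.
; Duplicate dancers or an early player trigger a radial impulse and red flash, while a winning player notifies the GameMode.
; Timelines animate per-slot target heights, which Tick follows with VInterpTo.
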(event OnComponentBeginOverlap(Capsule)
  (params (OverlappedComponent :type Primitive%20Component%20Object%20Reference) (OtherActor :type Actor%20Object%20Reference) (OtherComp :type Primitive%20Component%20Object%20Reference) (OtherBodyIndex :type Integer) (bFromSweep :type Boolean) (SweepResult :type Hit%20Result%20Structure%20%28by%20ref%29))
  (bind _asbp_ia_dancer_blue (Utilities|Casting|CastToBP_IA_Dancer_Blue OtherActor)
    (:then
      (Variables|/Game/ThirdPersonBP/Blueprints/AI/BP_IA_Dancer.BP_IA_Dancer_C|SetBP_EndDemo _asbp_ia_dancer_blue self)
      (bind _blueactor (Variables|Default|GetBlueActor)
        (:then
          (if (!= _blueactor _asbp_ia_dancer_blue)
            (CallFunction|CERepulse)))
        (:else
          (Utilities|FlowControl|DoOnce false
            (:Completed
              (Rendering|Components|Light|SetIntensity (Variables|/Script/Engine.SpotLight|GetSpotLightComponent (Variables|Default|GetBP_SpotLightBleu)) 1.6e+02)
              (CallFunction|AddBlueGuy)
              (EventDispatchers|AssignEVHasBeenDepossed _asbp_ia_dancer_blue (delegate Custom|EV_HasBeenDepossed_Event_1))
              (Default|RejectPawn _asbp_ia_dancer_blue)
              (Utilities|FlowControl|MultiGate false false -1 :!label _label
                (:Out%202
                  (Variables|Default|SetbIsWinnable? true))))))))
    (:CastFailed
      (bind _asbp_ia_dancer_yellow (Utilities|Casting|CastToBP_IA_Dancer_Yellow OtherActor)
        (:then
          (Variables|/Game/ThirdPersonBP/Blueprints/AI/BP_IA_Dancer.BP_IA_Dancer_C|SetBP_EndDemo _asbp_ia_dancer_yellow self)
          (bind _yellowactor (Variables|Default|GetYellowActor)
            (:then
              (if (!= _yellowactor _asbp_ia_dancer_yellow)
                (CallFunction|CERepulse)))
            (:else
              (Utilities|FlowControl|DoOnce false
                (:Completed
                  (Rendering|Components|Light|SetIntensity (Variables|/Script/Engine.SpotLight|GetSpotLightComponent (Variables|Default|GetBP_SpotLightJaune)) 1.6e+02)
                  (CallFunction|AddYellowGuy)
                  (EventDispatchers|AssignEVHasBeenDepossed _asbp_ia_dancer_yellow (delegate Custom|EV_HasBeenDepossed_Event_2))
                  (Default|RejectPawn _asbp_ia_dancer_yellow)
                  (goto _label))))))
        (:CastFailed
          (bind _asbp_ia_dancer_red (Utilities|Casting|CastToBP_IA_Dancer_Red OtherActor)
            (:then
              (Variables|/Game/ThirdPersonBP/Blueprints/AI/BP_IA_Dancer.BP_IA_Dancer_C|SetBP_EndDemo _asbp_ia_dancer_red self)
              (bind _redactor (Variables|Default|GetRedActor)
                (:then
                  (if (!= _redactor _asbp_ia_dancer_red)
                    (CallFunction|CERepulse)))
                (:else
                  (Utilities|FlowControl|DoOnce false
                    (:Completed
                      (Rendering|Components|Light|SetIntensity (Variables|/Script/Engine.SpotLight|GetSpotLightComponent (Variables|Default|GetBP_SpotLightRouge)) 1.6e+02)
                      (CallFunction|AddRedGuy)
                      (EventDispatchers|AssignEVHasBeenDepossed _asbp_ia_dancer_red (delegate Custom|EV_HasBeenDepossed_Event_0))
                      (Default|RejectPawn _asbp_ia_dancer_red)
                      (goto _label))))))
            (:CastFailed
              (bind _asthird_person_character (Utilities|Casting|CastToThirdPersonCharacter OtherActor))
              (if (Variables|Default|GetbIsWinnable?)
                (Utilities|FlowControl|DoOnce false
                  (:Completed
                    (Default|CallEVDemoFinished)
                    (Variables|Default|SetPlayerActor _asthird_person_character)
                    (CallFunction|AddPlayer)
                    (EventDispatchers|AssignEVSendActorEndDemo (Variables|Default|GetGameMode) (delegate Custom|EV_SendActorEndDemo_Event_0))
                    (Default|SetIsEndDemo (Variables|Default|GetGameMode))))
                (else
                  (CallFunction|CERepulse))))))))))

(event Custom|AddWhiteGuy
  (params (NewParam :type Actor%20Object%20Reference))
  (Variables|Default|SetWhiteActor NewParam)
  (Components|Timeline|SetPlayRate (Variables|Default|GetTimeline_0) 0.3)
  (bind _newtrack_0 (Timeline|Timeline_0 PlayFromStart)
    (:Update
      (Transformation|SetActorLocation (Variables|Default|GetWhiteActor) (+ (Math|Transform|TransformLocation (Transformation|GetActorTransform) (Variables|Default|GetWhiteGuyLoc)) (Math|Vector|MakeVector 0.0 0.0 _newtrack_0)) false false))))

(event Custom|AddRedGuy
  ;[1 1 1] Yello
  (Components|Timeline|SetPlayRate (Variables|Default|GetTimeline_3) 0.2)
  (bind _newtrack_0 (Timeline|Timeline_3 PlayFromStart)
    (:Update
      (Variables|Default|SetRedGuyLocFinalLoc (+ (Math|Transform|TransformLocation (Transformation|GetActorTransform) (Variables|Default|GetRedGuyLoc)) (Math|Vector|MakeVector 0.0 0.0 _newtrack_0))))))

(event Custom|EV_HasBeenDepossed_Event_0
  (params (NewActorCreated :type Actor%20Object%20Reference))
  (bind _output_get (Variables|Default|SetRedActor NewActorCreated))
  (EventDispatchers|UnbindEventfromEVHasBeenDepossed (stale OnComponentBeginOverlap(Capsule) _asbp_ia_dancer_red) (delegate Custom|EV_HasBeenDepossed_Event_0))
  (Transformation|SetActorRotation _output_get "0,-180.000000, 0"))

(event Custom|EV_SendActorEndDemo_Event_0
  (params (ActorToCheck :type Actor%20Object%20Reference))
  (bind _asbp_ia_dancer_blue (Utilities|Casting|CastToBP_IA_Dancer_Blue ActorToCheck)
    (:then
      (Variables|Default|SetBlueActor _asbp_ia_dancer_blue))
    (:CastFailed
      (bind _asbp_ia_dancer_yellow (Utilities|Casting|CastToBP_IA_Dancer_Yellow ActorToCheck)
        (:then
          (Variables|Default|SetYellowActor _asbp_ia_dancer_yellow))
        (:CastFailed
          (bind _asbp_ia_dancer_red (Utilities|Casting|CastToBP_IA_Dancer_Red ActorToCheck)
            (:then
              (Variables|Default|SetRedActor _asbp_ia_dancer_red))
            (:CastFailed
              (bind _asbp_ia_dancer_no_name (Utilities|Casting|CastToBP_IA_Dancer_NoName ActorToCheck)
                (:then
                  (Variables|Default|SetWhiteActor _asbp_ia_dancer_no_name))
                (:CastFailed
                  (bind _asthird_person_character (Utilities|Casting|CastToThirdPersonCharacter ActorToCheck))
                  (Variables|Default|SetPlayerActor _asthird_person_character))))))))))

(event Custom|EV_HasBeenDepossed_Event_1
  (params (NewActorCreated :type Actor%20Object%20Reference))
  (bind _output_get (Variables|Default|SetBlueActor NewActorCreated))
  (EventDispatchers|UnbindEventfromEVHasBeenDepossed (stale OnComponentBeginOverlap(Capsule) _asbp_ia_dancer_blue) (delegate Custom|EV_HasBeenDepossed_Event_1))
  (Transformation|SetActorRotation _output_get "0,-180.000000, 0"))

(event Custom|EV_HasBeenDepossed_Event_2
  (params (NewActorCreated :type Actor%20Object%20Reference))
  (bind _output_get (Variables|Default|SetYellowActor NewActorCreated))
  (EventDispatchers|UnbindEventfromEVHasBeenDepossed (stale OnComponentBeginOverlap(Capsule) _asbp_ia_dancer_yellow) (delegate Custom|EV_HasBeenDepossed_Event_2))
  (Transformation|SetActorRotation _output_get "0,-180.000000, 0"))

(event Custom|AddBlueGuy
  ;[1 1 1] Blue
  (Components|Timeline|SetPlayRate (Variables|Default|GetTimeline_1) 0.2)
  (bind _newtrack_0 (Timeline|Timeline_1 PlayFromStart)
    (:Update
      (Variables|Default|SetBlueGuyLocFinalLoc (+ (Math|Transform|TransformLocation (Transformation|GetActorTransform) (Variables|Default|GetBlueGuyLoc)) (Math|Vector|MakeVector 0.0 0.0 _newtrack_0))))))

(event Custom|CE_Repulse
  (Class|RadialForceComponent|FireImpulse (Variables|Default|GetRadialForce))
  (Rendering|Components|Light|SetLightColor (Variables|/Script/Engine.Light|GetLightComponent (Variables|Default|GetSpotlightCentral)) "(R=1.000000,G=0.000000,B=0.000000,A=1.000000)" true)
  (Utilities|FlowControl|Delay 0.2)
  (Rendering|Components|Light|SetLightColor (Variables|/Script/Engine.Light|GetLightComponent (Variables|Default|GetSpotlightCentral)) "(R=1.000000,G=1.000000,B=1.000000,A=1.000000)" true)
  (Utilities|FlowControl|Delay 0.5))

(event Custom|AddYellowGuy
  ;[1 1 1] Yello
  (Components|Timeline|SetPlayRate (Variables|Default|GetTimeline_2) 0.2)
  (bind _newtrack_0 (Timeline|Timeline_2 PlayFromStart)
    (:Update
      (Variables|Default|SetYellowGuyLocFinalLoc (+ (Math|Transform|TransformLocation (Transformation|GetActorTransform) (Variables|Default|GetYellowGuyLoc)) (Math|Vector|MakeVector 0.0 0.0 _newtrack_0))))))

(event Custom|AddPlayer
  ;[1 1 1] Yello
  (Components|Timeline|SetPlayRate (Variables|Default|GetTimeline_4) 0.2)
  (bind _newtrack_0 (Timeline|Timeline_4 PlayFromStart)
    (:Update
      (Variables|Default|SetPlayerLocFinal (+ (Math|Transform|TransformLocation (Transformation|GetActorTransform) (Variables|Default|GetPlayerLoc)) (Math|Vector|MakeVector 0.0 0.0 _newtrack_0))))))

(event EventBeginPlay
  (bind _asthird_person_game_mode (Utilities|Casting|CastToThirdPersonGameMode (Game|GetGameMode)))
  (Variables|Default|SetGameMode _asthird_person_game_mode))

(event Collision|EventActorBeginOverlap
  (params (OtherActor :type Actor%20Object%20Reference)))

(event EventTick
  (params (DeltaSeconds :type Float%20%28single-precision%29))
  (Utilities|FlowControl|Sequence
    (:then_0
      (bind _blueactor (Variables|Default|GetBlueActor)
        (:then
          (Transformation|SetActorLocation _blueactor (Math|Interpolation|VInterpTo (Transformation|GetActorLocation _blueactor) (Variables|Default|GetBlueGuyLocFinalLoc) (Utilities|Time|GetWorldDeltaSeconds) 2e+01) false true))
        (:else)))
    (:then_1
      (bind _yellowactor (Variables|Default|GetYellowActor)
        (:then
          (Transformation|SetActorLocation _yellowactor (Math|Interpolation|VInterpTo (Transformation|GetActorLocation _yellowactor) (Variables|Default|GetYellowGuyLocFinalLoc) (Utilities|Time|GetWorldDeltaSeconds) 2e+01) false true))
        (:else)))
    (:then_2
      (bind _redactor (Variables|Default|GetRedActor)
        (:then
          (Transformation|SetActorLocation _redactor (Math|Interpolation|VInterpTo (Transformation|GetActorLocation _redactor) (Variables|Default|GetRedGuyLocFinalLoc) (Utilities|Time|GetWorldDeltaSeconds) 2e+01) false true))
        (:else)))
    (:then_3
      (bind _playeractor (Variables|Default|GetPlayerActor)
        (:then
          (Transformation|SetActorLocation _playeractor (Math|Interpolation|VInterpTo (Transformation|GetActorLocation _playeractor) (Variables|Default|GetPlayerLocFinal) (Utilities|Time|GetWorldDeltaSeconds) 2e+01) false true))
        (:else)))))

(fn ConstructionScript)