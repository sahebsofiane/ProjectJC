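; Strobe light Blueprint that flashes a spot light and swings it in random directions.
; On BeginPlay a randomly delayed timeline switches light intensity fully on or off, replaying at a new random play rate each time it finishes.
; In parallel, delay loops randomize the RotatingMovement rotation rate and reapply a constant white color at random intervals.
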(event EventBeginPlay
  (Utilities|FlowControl|Sequence
    (:then_0
      (Rendering|Components|Light|SetLightColor (Variables|Default|GetSpotLightComponent) "(R=1.000000,G=1.000000,B=1.000000,A=1.000000)" true :!label _label)
      (Utilities|FlowControl|Delay (Math|Random|RandomFloatinRange 1.0 3.0))
      (goto _label))
    (:then_1
      (Utilities|FlowControl|Delay (Math|Random|RandomFloatinRange 0.2 1.0))
      (bind _newtrack_0 (Timeline|Timeline_0 PlayFromStart)
        (:Update
          (Rendering|Components|Light|SetIntensity (Variables|Default|GetLightComponent) (select (== _newtrack_0 0.0) 0.0 1.6e+02)))
        (:Finished
          (Components|Timeline|SetPlayRate (Variables|Default|GetTimeline_0) (Math|Random|RandomFloatinRange 0.8 2.0))
          (Timeline|Timeline_0 PlayFromStart))))
    (:then_2
      (Variables|/Script/Engine.RotatingMovementComponent|SetRotationRate (Variables|Default|GetRotatingMovement) (Math|Random|RandomRotator true) :!label _label_2)
      (Utilities|FlowControl|Delay (Math|Random|RandomFloatinRange 0.5 1.25))
      (goto _label_2))))

(event EventTick
  (params (DeltaSeconds :type Float%20%28single-precision%29)))

(fn ConstructionScript)