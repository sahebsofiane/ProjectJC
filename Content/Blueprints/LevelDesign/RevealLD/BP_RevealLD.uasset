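; BP_RevealLD is a hidden level-design mesh that the Yellow Dancer's power reveals and makes solid.
; Construction gives the mesh and its children dynamic materials; BeginPlay hides them and ignores Pawn collision on the root.
; Trigger overlap binds the power event and fades opacity; a timer also fades it once the player controls that dancer.
; Revealing destroys BlockVolumes, animates opacity and emissive, restores collision, then applies RampMaterial; Mojo graphs are unused.
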(event OnActorBeginOverlap(TriggerVolume)
  (params (OverlappedActor :type Actor%20Object%20Reference) (OtherActor :type Actor%20Object%20Reference))
  (bind _asbp_ia_dancer_yellow (Utilities|Casting|CastToBP_IA_Dancer_Yellow OtherActor))
  (bind _output_get (Variables|Default|SetYellowDancerRef _asbp_ia_dancer_yellow))
  (EventDispatchers|AssignEVUsingPower _output_get (delegate Custom|EV_UsingPower_Event_0))
  (bind _newtrack_0 (Timeline|Timeline_2 PlayFromStart)
    (:Update
      (for _array_element (Variables|Default|GetDMI_Array)
        (Rendering|Material|SetScalarParameterValue _array_element "Opacity" _newtrack_0 :!class /Script/Engine.MaterialInstanceDynamic)))))

(event OnActorEndOverlap(TriggerVolume)
  (params (OverlappedActor :type Actor%20Object%20Reference) (OtherActor :type Actor%20Object%20Reference))
  (bind _asbp_ia_dancer_yellow (Utilities|Casting|CastToBP_IA_Dancer_Yellow OtherActor))
  (EventDispatchers|UnbindEventfromEVUsingPower _asbp_ia_dancer_yellow (delegate Custom|EV_UsingPower_Event_0))
  (Variables|Default|SetYellowDancerRef 0)
  (bind _newtrack_0 (Timeline|Timeline_2 Reverse)
    (:Update
      (for _array_element (Variables|Default|GetDMI_Array)
        (Rendering|Material|SetScalarParameterValue _array_element "Opacity" _newtrack_0 :!class /Script/Engine.MaterialInstanceDynamic)))))

(event Custom|EV_UsingPower_Event_0
  (params (AvailableMana :type Float%20%28single-precision%29))
  (CallFunction|CERevealMesh))

(event Custom|EV_UsingPower_Event_1
  (params (AvailableMana :type Float%20%28single-precision%29))
  (CallFunction|CERevealMesh))

(event Custom|CE_RevealMesh
  (bind _staticmesh (Variables|Default|GetStaticMesh))
  (for _array_element (Variables|Default|GetBlockVolumes)
    (Actor|DestroyActor _array_element))
  (bind _newtrack_0 (Timeline|Timeline_1 PlayFromStart)
    (:Update
      (for _array_element_2 (Variables|Default|GetDMI_Array)
        (Rendering|Material|SetScalarParameterValue _array_element_2 "Opacity" _newtrack_0 :!class /Script/Engine.MaterialInstanceDynamic)))
    (:NewTrack_1
      (Collision|SetCollisionResponsetoChannel _staticmesh "ECC_Pawn" "ECR_Block")
      (Collision|SetCollisionResponsetoChannel _staticmesh "ECC_PhysicsBody" "ECR_Block")
      (for _array_element_3 (Components|GetChildrenComponents (Variables|Default|GetStaticMesh) true)
        (bind _asstatic_mesh_component (Utilities|Casting|CastToStaticMeshComponent _array_element_3))
        (Collision|SetCollisionResponsetoChannel _asstatic_mesh_component "ECC_Pawn" "ECR_Block"))
      (bind _emissive (Timeline|Timeline_0 PlayFromStart)
        (:Update
          (for _array_element_4 (Variables|Default|GetDMI_Array)
            (Rendering|Material|SetScalarParameterValue _array_element_4 "Emissive" _emissive :!class /Script/Engine.MaterialInstanceDynamic)))
        (:Finished
          (Rendering|Material|SetMaterial (Variables|Default|GetStaticMesh) 0 "/Game/ThirdPerson/Meshes/RampMaterial.RampMaterial")
          (for _array_element_5 (Components|GetChildrenComponents (Variables|Default|GetStaticMesh) true)
            (bind _asstatic_mesh_component_2 (Utilities|Casting|CastToStaticMeshComponent _array_element_5))
            (Rendering|Material|SetMaterial _asstatic_mesh_component_2 0 "/Game/ThirdPerson/Meshes/RampMaterial.RampMaterial")))))))

(event Custom|CustomEvent_0
  (Utilities|Casting|CastToBP_IA_Dancer_Yellow (Game|Player|GetPlayerPawn 0))
  (Utilities|Time|ClearandInvalidateTimerbyHandle (Variables|Default|GetTimerHandleCheckControlledPawn))
  (bind _newtrack_0 (Timeline|Timeline_2 PlayFromStart)
    (:Update
      (for _array_element (Variables|Default|GetDMI_Array)
        (Rendering|Material|SetScalarParameterValue _array_element "Opacity" _newtrack_0 :!class /Script/Engine.MaterialInstanceDynamic)))))

(event EventBeginPlay
  (CallFunction|Init)
  (bind _yellowdancerref (Variables|Default|GetYellowDancerRef)
    (:then
      (EventDispatchers|AssignEVUsingPower _yellowdancerref (delegate Custom|EV_UsingPower_Event_1))
      (bind _returnvalue (Utilities|Time|SetTimerbyEvent (delegate Custom|CustomEvent_0) 0.2 true))
      (Variables|Default|SetTimerHandleCheckControlledPawn _returnvalue))
    (:else)))

(event Collision|EventActorBeginOverlap
  (params (OtherActor :type Actor%20Object%20Reference)))

(event EventTick
  (params (DeltaSeconds :type Float%20%28single-precision%29))
  (Variables|Default|SetDeltaTime DeltaSeconds))

(fn ConstructionScript
  (bind _staticmesh (Variables|Default|GetStaticMesh))
  (Utilities|Array|Clear (Variables|Default|GetDMI_Array))
  (Rendering|Material|SetMaterial _staticmesh 0 "/Game/Blueprints/LevelDesign/RevealLD/MA_RevealID.MA_RevealID")
  (bind _returnvalue (Rendering|Material|CreateDynamicMaterialInstance _staticmesh 0 "/Game/Blueprints/LevelDesign/RevealLD/MA_RevealID.MA_RevealID" "None" :!class /Script/Engine.PrimitiveComponent))
  (Utilities|Array|AddUnique (Variables|Default|GetDMI_Array) _returnvalue)
  (for _array_element (Components|GetChildrenComponents (Variables|Default|GetStaticMesh) true)
    (bind _asstatic_mesh_component (Utilities|Casting|CastToStaticMeshComponent _array_element))
    (Rendering|Material|SetMaterial _asstatic_mesh_component 0 "/Game/Blueprints/LevelDesign/RevealLD/MA_RevealID.MA_RevealID")
    (bind _returnvalue_2 (Rendering|Material|CreateDynamicMaterialInstance _asstatic_mesh_component 0 "/Game/Blueprints/LevelDesign/RevealLD/MA_RevealID.MA_RevealID" "None" :!class /Script/Engine.PrimitiveComponent))
    (Utilities|Array|AddUnique (Variables|Default|GetDMI_Array) _returnvalue_2))
  (for _array_element_2 (Variables|Default|GetDMI_Array)
    (Rendering|Material|SetScalarParameterValue _array_element_2 "Emissive" (Variables|Default|GetEmissive) :!class /Script/Engine.MaterialInstanceDynamic)
    (Rendering|Material|SetScalarParameterValue _array_element_2 "Opacity" (Variables|Default|GetOpacity) :!class /Script/Engine.MaterialInstanceDynamic)))

(fn Init
  (Collision|SetCollisionResponsetoChannel (Variables|Default|GetStaticMesh) "ECC_Pawn" "ECR_Ignore")
  (for _array_element (Variables|Default|GetDMI_Array)
    (Rendering|Material|SetScalarParameterValue _array_element "Opacity" 0.0 :!class /Script/Engine.MaterialInstanceDynamic)))