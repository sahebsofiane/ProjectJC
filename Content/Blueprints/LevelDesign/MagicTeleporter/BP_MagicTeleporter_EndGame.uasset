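; End-game variant of the magic teleporter, whose Begin and End trigger boxes, while OverrideActive, move overlapping actors elsewhere.
; Each box's settings target either an override actor, with a spline-actor camera blend, or a linked teleporter's Begin or End point.
; Linked jumps hand the active state and spotlight to the destination, whose Tick slides the light along its spline toward the player.
; The End box can also trigger the player's memory-stick handling.
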(event OnComponentBeginOverlap(BoxBegin)
  (params (OverlappedComponent :type Primitive%20Component%20Object%20Reference) (OtherActor :type Actor%20Object%20Reference) (OtherComp :type Primitive%20Component%20Object%20Reference) (OtherBodyIndex :type Integer) (bFromSweep :type Boolean) (SweepResult :type Hit%20Result%20Structure%20%28by%20ref%29))
  (bind _bp_magicteleporterstart (Variables|Default|GetBP_MagicTelePorterStart))
  (bind _overriderotation (Variables|Default|GetOverrideRotation))
  (bind (_magicteleporter _positiononmagicteleporter _memorystick_ _overrideactorposition _splineactor) (Utilities|Struct|BreakSTR_MagicTeleporterRef _bp_magicteleporterstart))
  (bind _returnvalue (Transformation|GetActorTransform _overrideactorposition))
  (bind _begin (Variables|/Game/Blueprints/LevelDesign/MagicTeleporter/BP_MagicTeleporter.BP_MagicTeleporter_C|GetBegin _magicteleporter))
  (bind _end (Variables|/Game/Blueprints/LevelDesign/MagicTeleporter/BP_MagicTeleporter.BP_MagicTeleporter_C|GetEnd _magicteleporter))
  (bind _returnvalue_2 (Transformation|GetWorldTransform _begin))
  (bind _returnvalue_3 (Transformation|GetWorldTransform _end))
  (bind (_location _rotation) (Math|Transform|BreakTransform _returnvalue))
  ;[0 0 0] Begin Teleportation
  (if (Variables|Default|GetOverrideActive)
    (Variables|Default|SetActorOverlaped OtherActor)
    (Utilities|IsValid _overrideactorposition
      (:Is%20Valid
        (Rendering|Debug|DrawDebugSphere _location 1e+01 12 "(R=1.000000,G=1.000000,B=1.000000,A=1.000000)" 2.0 1e+01)
        (Transformation|SetActorLocationAndRotation (Variables|Default|GetActorOverlaped) _location _rotation)
        (Utilities|IsValid _splineactor
          (:Is%20Valid
            (Default|OverrideBlendCam _splineactor))))
      (:Is%20Not%20Valid
        (Rendering|SetVisibility (Variables|/Game/Blueprints/LevelDesign/MagicTeleporter/BP_MagicTeleporter.BP_MagicTeleporter_C|GetSpotLight _magicteleporter) true false)
        (Variables|/Game/Blueprints/LevelDesign/MagicTeleporter/BP_MagicTeleporter.BP_MagicTeleporter_C|SetIsTeleporterActive? _magicteleporter true)
        (switch Utilities|FlowControl|Switch|SwitchonEN_MagicTeleporterPlacement _positiononmagicteleporter
          (:NewEnumerator0
            (Transformation|SetActorLocationAndRotation (Variables|Default|GetActorOverlaped) (.location _returnvalue_2) (select _overriderotation "0, 0, 0" (.rotation _returnvalue_2)) false true))
          (:NewEnumerator1
            (Transformation|SetActorLocationAndRotation (Variables|Default|GetActorOverlaped) (.location _returnvalue_3) (select _overriderotation "0, 0, 0" (.rotation _returnvalue_3)) false true)))
        (if (not (== _magicteleporter self))
          (Variables|Default|SetIsTeleporterActive? false)
          (Rendering|SetVisibility (Variables|Default|GetSpotLight) false false))))))

(event OnComponentBeginOverlap(BoxEnd)
  (params (OverlappedComponent :type Primitive%20Component%20Object%20Reference) (OtherActor :type Actor%20Object%20Reference) (OtherComp :type Primitive%20Component%20Object%20Reference) (OtherBodyIndex :type Integer) (bFromSweep :type Boolean) (SweepResult :type Hit%20Result%20Structure%20%28by%20ref%29))
  (bind _bp_magicteleporterend (Variables|Default|GetBP_MagicTelePorterEnd))
  (bind _overriderotation (Variables|Default|GetOverrideRotation))
  (bind (_magicteleporter _positiononmagicteleporter _memorystick_ _overrideactorposition _splineactor) (Utilities|Struct|BreakSTR_MagicTeleporterRef _bp_magicteleporterend))
  (bind _returnvalue (Transformation|GetActorTransform _overrideactorposition))
  (bind _end (Variables|/Game/Blueprints/LevelDesign/MagicTeleporter/BP_MagicTeleporter.BP_MagicTeleporter_C|GetEnd _magicteleporter))
  (bind _begin (Variables|/Game/Blueprints/LevelDesign/MagicTeleporter/BP_MagicTeleporter.BP_MagicTeleporter_C|GetBegin _magicteleporter))
  (bind (_location _rotation) (Math|Transform|BreakTransform _returnvalue))
  (bind _returnvalue_2 (Transformation|GetWorldTransform _begin))
  (bind _returnvalue_3 (Transformation|GetWorldTransform _end))
  ;[0 0 0] End Teleportaton
  (if (Variables|Default|GetOverrideActive)
    (Variables|Default|SetActorOverlaped OtherActor)
    (Utilities|FlowControl|Sequence
      (:then_0
        (if _memorystick_
          (bind _asthird_person_character (Utilities|Casting|CastToThirdPersonCharacter (Game|Player|GetPlayerPawn 0)))
          (Default|MemoryStickHandle _asthird_person_character)))
      (:then_1
        (Utilities|IsValid _overrideactorposition
          (:Is%20Valid
            (Transformation|SetActorLocationAndRotation (Variables|Default|GetActorOverlaped) _location _rotation false true)
            (Default|OverrideBlendCam _splineactor))
          (:Is%20Not%20Valid
            (Rendering|SetVisibility (Variables|/Game/Blueprints/LevelDesign/MagicTeleporter/BP_MagicTeleporter.BP_MagicTeleporter_C|GetSpotLight _magicteleporter) true false)
            (Variables|/Game/Blueprints/LevelDesign/MagicTeleporter/BP_MagicTeleporter.BP_MagicTeleporter_C|SetIsTeleporterActive? _magicteleporter true)
            (switch Utilities|FlowControl|Switch|SwitchonEN_MagicTeleporterPlacement _positiononmagicteleporter
              (:NewEnumerator0
                (Transformation|SetActorLocationAndRotation (Variables|Default|GetActorOverlaped) (.location _returnvalue_2) (select _overriderotation "0, 0, 0" (.rotation _returnvalue_2)) false true))
              (:NewEnumerator1
                (Transformation|SetActorLocationAndRotation (Variables|Default|GetActorOverlaped) (.location _returnvalue_3) (select _overriderotation "0, 0, 0" (.rotation _returnvalue_3)) false true)))
            (if (not (== _magicteleporter self))
              (Variables|Default|SetIsTeleporterActive? false)
              (Rendering|SetVisibility (Variables|Default|GetSpotLight) false false))))))))

(event Collision|EventActorBeginOverlap
  (params (OtherActor :type Actor%20Object%20Reference)))

(event EventTick
  (params (DeltaSeconds :type Float%20%28single-precision%29))
  (if (and (Variables|Default|GetIsTeleporterActive?) (Variables|Default|GetOverrideActive))
    (Transformation|SetWorldLocation (Variables|Default|GetSpotLight) (Spline|FindLocationClosesttoWorldLocation (Variables|Default|GetSpline) (Transformation|GetActorLocation (Game|Player|GetPlayerPawn 0)) "World") false false)))

(fn ConstructionScript
  (Rendering|SetVisibility (Variables|Default|GetSpotLight) (Variables|Default|GetIsTeleporterActive?) false))