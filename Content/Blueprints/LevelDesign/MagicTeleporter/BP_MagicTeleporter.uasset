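; Magic teleporter actor with Begin and End trigger boxes that move the player to the Begin or End point of a configured teleporter.
; Each box's link struct picks target teleporter and position, and can trigger MemoryStickHandle on the ThirdPersonCharacter.
; Teleporting activates the target and its spotlight, switching this one off if different.
; While active, Tick keeps the spotlight at the spline point closest to the player.
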(event OnComponentBeginOverlap(BoxBegin)
  (params (OverlappedComponent :type Primitive%20Component%20Object%20Reference) (OtherActor :type Actor%20Object%20Reference) (OtherComp :type Primitive%20Component%20Object%20Reference) (OtherBodyIndex :type Integer) (bFromSweep :type Boolean) (SweepResult :type Hit%20Result%20Structure%20%28by%20ref%29))
  (bind _returnvalue (Game|Player|GetPlayerPawn 0))
  (bind _bp_magicteleporterstart (Variables|Default|GetBP_MagicTelePorterStart))
  (bind (_magicteleporter _positiononmagicteleporter _memorystick_) (Utilities|Struct|BreakSTR_MagicTeleporterRef _bp_magicteleporterstart))
  (bind _begin (Variables|BP_MagicTeleporter_C|GetBegin _magicteleporter))
  (bind _end (Variables|BP_MagicTeleporter_C|GetEnd _magicteleporter))
  (bind _returnvalue_2 (Transformation|GetWorldTransform _begin))
  (bind _returnvalue_3 (Transformation|GetWorldTransform _end))
  ;[0 0 0] Begin Teleportation
  (if (== OtherActor (Game|Player|GetPlayerPawn 0))
    (Utilities|FlowControl|Sequence
      (:then_0
        (if _memorystick_
          (bind _asthird_person_character (Utilities|Casting|CastToThirdPersonCharacter (Game|Player|GetPlayerPawn 0)))
          (Default|MemoryStickHandle _asthird_person_character)))
      (:then_1
        (Rendering|SetVisibility (Variables|BP_MagicTeleporter_C|GetSpotLight _magicteleporter) true false)
        (Variables|BP_MagicTeleporter_C|SetIsTeleporterActive? _magicteleporter true)
        (switch Utilities|FlowControl|Switch|SwitchonEN_MagicTeleporterPlacement _positiononmagicteleporter
          (:NewEnumerator0
            (Transformation|SetActorLocationAndRotation _returnvalue (.location _returnvalue_2) (.rotation _returnvalue_2) false true))
          (:NewEnumerator1
            (Transformation|SetActorLocationAndRotation _returnvalue (.location _returnvalue_3) (.rotation _returnvalue_3) false true)))
        (if (not (== _magicteleporter self))
          (Variables|Default|SetIsTeleporterActive? false)
          (Rendering|SetVisibility (Variables|Default|GetSpotLight) false false))))))

(event OnComponentBeginOverlap(BoxEnd)
  (params (OverlappedComponent :type Primitive%20Component%20Object%20Reference) (OtherActor :type Actor%20Object%20Reference) (OtherComp :type Primitive%20Component%20Object%20Reference) (OtherBodyIndex :type Integer) (bFromSweep :type Boolean) (SweepResult :type Hit%20Result%20Structure%20%28by%20ref%29))
  (bind _returnvalue (Game|Player|GetPlayerPawn 0))
  (bind _bp_magicteleporterend (Variables|Default|GetBP_MagicTelePorterEnd))
  (bind (_magicteleporter _positiononmagicteleporter _memorystick_) (Utilities|Struct|BreakSTR_MagicTeleporterRef _bp_magicteleporterend))
  (bind _end (Variables|BP_MagicTeleporter_C|GetEnd _magicteleporter))
  (bind _begin (Variables|BP_MagicTeleporter_C|GetBegin _magicteleporter))
  (bind _returnvalue_2 (Transformation|GetWorldTransform _begin))
  (bind _returnvalue_3 (Transformation|GetWorldTransform _end))
  ;[0 0 0] End Teleportaton
  (if (== OtherActor (Game|Player|GetPlayerPawn 0))
    (Utilities|FlowControl|Sequence
      (:then_0
        (if _memorystick_
          (bind _asthird_person_character (Utilities|Casting|CastToThirdPersonCharacter (Game|Player|GetPlayerPawn 0)))
          (Default|MemoryStickHandle _asthird_person_character)))
      (:then_1
        (Rendering|SetVisibility (Variables|BP_MagicTeleporter_C|GetSpotLight _magicteleporter) true false)
        (Variables|BP_MagicTeleporter_C|SetIsTeleporterActive? _magicteleporter true)
        (switch Utilities|FlowControl|Switch|SwitchonEN_MagicTeleporterPlacement _positiononmagicteleporter
          (:NewEnumerator0
            (Transformation|SetActorLocationAndRotation _returnvalue (.location _returnvalue_2) (.rotation _returnvalue_2) false true))
          (:NewEnumerator1
            (Transformation|SetActorLocationAndRotation _returnvalue (.location _returnvalue_3) (.rotation _returnvalue_3) false true)))
        (if (not (== _magicteleporter self))
          (Variables|Default|SetIsTeleporterActive? false)
          (Rendering|SetVisibility (Variables|Default|GetSpotLight) false false))))))

(event EventBeginPlay
  (bind _bp_magicteleporterend (Variables|Default|GetBP_MagicTelePorterEnd))
  (bind _bp_magicteleporterstart (Variables|Default|GetBP_MagicTelePorterStart))
  (bind (_magicteleporter _positiononmagicteleporter _memorystick_) (Utilities|Struct|BreakSTR_MagicTeleporterRef _bp_magicteleporterstart))
  (bind (_magicteleporter_2 _positiononmagicteleporter_2 _memorystick__2) (Utilities|Struct|BreakSTR_MagicTeleporterRef _bp_magicteleporterend))
  (Variables|Default|SetEndActor _magicteleporter_2)
  (Variables|Default|SetEndEnum _positiononmagicteleporter_2)
  (Variables|Default|SetEndStickMemory _memorystick__2)
  (Variables|Default|SetBeginActor _magicteleporter)
  (Variables|Default|SetStartEnum _positiononmagicteleporter)
  (Variables|Default|SetStartStickMemory _memorystick_))

(event Collision|EventActorBeginOverlap
  (params (OtherActor :type Actor%20Object%20Reference)))

(event EventTick
  (params (DeltaSeconds :type Float%20%28single-precision%29))
  (if (Variables|Default|GetIsTeleporterActive?)
    (Transformation|SetWorldLocation (Variables|Default|GetSpotLight) (Spline|FindLocationClosesttoWorldLocation (Variables|Default|GetSpline) (Transformation|GetActorLocation (Game|Player|GetPlayerPawn 0)) "World") false false)))

(fn ConstructionScript
  (Rendering|SetVisibility (Variables|Default|GetSpotLight) (Variables|Default|GetIsTeleporterActive?) false))