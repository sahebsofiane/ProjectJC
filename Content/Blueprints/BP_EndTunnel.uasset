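; BP_EndTunnel is an actor that repeatedly moves its StaticMeshOne component along world Z, apparently as a moving end-tunnel effect.
; On BeginPlay it caches the mesh's actor location, then a timeline lerps from there toward a point 100,000 units higher.
; An event track on the same timeline restarts playback from the start after a short delay, so the movement loops from the original position.
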(event EventBeginPlay
  (Variables|Default|SetOriginLocation (Transformation|GetActorLocation (Variables|Default|GetStaticMeshOne)))
  (bind _newtrack_1 (Timeline|Timeline_0 PlayFromStart)
    (:Update
      (Transformation|SetActorLocation (Variables|Default|GetStaticMeshOne) (Math|Vector|Lerp(Vector) (Variables|Default|GetOriginLocation) (+ (Variables|Default|GetOriginLocation) "0, 0,100000.000000") _newtrack_1) false false))
    (:NewTrack_2
      (Utilities|FlowControl|Delay 0.2)
      (Timeline|Timeline_0 PlayFromStart))))

(event Collision|EventActorBeginOverlap
  (params (OtherActor :type Actor%20Object%20Reference)))

(event EventTick
  (params (DeltaSeconds :type Float%20%28single-precision%29)))

(fn ConstructionScript)