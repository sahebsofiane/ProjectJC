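; Cube_DM_Blueprint is a destructible cube actor that cleans itself up after it breaks.
; When its DestructibleComponent fractures, it enables physics simulation, waits a few seconds, then destroys the actor.
; The construction script creates dynamic material instances for both material slots and sets their Opacity parameter to fully opaque, though nothing in the graph changes it afterward.
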(event OnComponentFracture(DestructibleComponent)
  (params (HitPoint :type Vector%20%28by%20ref%29 :default "0, 0, 0") (HitDirection :type Vector%20%28by%20ref%29 :default "0, 0, 0"))
  (Physics|SetSimulatePhysics (Variables|Default|GetDestructibleComponent) true)
  (Utilities|FlowControl|Delay 3.0)
  (Actor|DestroyActor))

(event EventBeginPlay)

(event Collision|EventActorBeginOverlap
  (params (OtherActor :type Actor%20Object%20Reference)))

(event EventTick
  (params (DeltaSeconds :type Float%20%28single-precision%29)))

(fn ConstructionScript
  (bind _destructiblecomponent (Variables|Default|GetDestructibleComponent))
  (bind _returnvalue (Rendering|Material|CreateDynamicMaterialInstance _destructiblecomponent 0 (Rendering|Material|GetMaterial _destructiblecomponent 0) "None" :!class /Script/Engine.PrimitiveComponent))
  (Variables|Default|SetDMI_0 _returnvalue)
  (bind _returnvalue_2 (Rendering|Material|CreateDynamicMaterialInstance _destructiblecomponent 1 (Rendering|Material|GetMaterial _destructiblecomponent 1) "None" :!class /Script/Engine.PrimitiveComponent))
  (Variables|Default|SetDMi_1 _returnvalue_2)
  (for _array_element (Utilities|Array|MakeArray (Variables|Default|GetDMI_0) (Variables|Default|GetDMi_1))
    (Rendering|Material|SetScalarParameterValue _array_element "Opacity" 1.0 :!class /Script/Engine.MaterialInstanceDynamic)))