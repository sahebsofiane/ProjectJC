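; Spline rail camera that moves an assigned camera along its spline to track the player, or the average of choice-mode actors when that mode is on.
; Tick interpolates toward the closest spline point, optionally adding a distance-based X offset and look-at rotation.
; Four trigger boxes or OverrideBlendCam blend the view to it and register it in the GameMode.
; One instance can be flagged as the instant starting camera, and construction previews placement via DebugTime.
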(event OnComponentBeginOverlap(Box)
  (params (OverlappedComponent :type Primitive%20Component%20Object%20Reference) (OtherActor :type Actor%20Object%20Reference) (OtherComp :type Primitive%20Component%20Object%20Reference) (OtherBodyIndex :type Integer) (bFromSweep :type Boolean) (SweepResult :type Hit%20Result%20Structure%20%28by%20ref%29))
  (Variables|Default|SetBlendTime (Variables|Default|GetCustomBlendTime))
  (Game|Player|SetViewTargetwithBlend (Game|GetPlayerController 0) (stale EventBeginPlay _cameravariable) (Variables|Default|GetBlendTime) "VTBlend_EaseInOut" 3.0 false)
  (Variables|/Game/ThirdPersonBP/Blueprints/ThirdPersonGameMode.ThirdPersonGameMode_C|SetBP_SplineCamera (Variables|Default|GetGameMode) self))

(event OnComponentBeginOverlap(Box1)
  (params (OverlappedComponent :type Primitive%20Component%20Object%20Reference) (OtherActor :type Actor%20Object%20Reference) (OtherComp :type Primitive%20Component%20Object%20Reference) (OtherBodyIndex :type Integer) (bFromSweep :type Boolean) (SweepResult :type Hit%20Result%20Structure%20%28by%20ref%29))
  (Variables|Default|SetBlendTime (Variables|Default|GetCustomBlendTime))
  (Game|Player|SetViewTargetwithBlend (Game|GetPlayerController 0) (stale EventBeginPlay _cameravariable) (Variables|Default|GetBlendTime) "VTBlend_EaseInOut" 3.0 false)
  (Variables|/Game/ThirdPersonBP/Blueprints/ThirdPersonGameMode.ThirdPersonGameMode_C|SetBP_SplineCamera (Variables|Default|GetGameMode) self))

(event OnComponentBeginOverlap(Box2)
  (params (OverlappedComponent :type Primitive%20Component%20Object%20Reference) (OtherActor :type Actor%20Object%20Reference) (OtherComp :type Primitive%20Component%20Object%20Reference) (OtherBodyIndex :type Integer) (bFromSweep :type Boolean) (SweepResult :type Hit%20Result%20Structure%20%28by%20ref%29))
  (Variables|Default|SetBlendTime (Variables|Default|GetCustomBlendTime))
  (Game|Player|SetViewTargetwithBlend (Game|GetPlayerController 0) (stale EventBeginPlay _cameravariable) (Variables|Default|GetBlendTime) "VTBlend_EaseInOut" 3.0 false)
  (Variables|/Game/ThirdPersonBP/Blueprints/ThirdPersonGameMode.ThirdPersonGameMode_C|SetBP_SplineCamera (Variables|Default|GetGameMode) self))

(event OnComponentBeginOverlap(Box3)
  (params (OverlappedComponent :type Primitive%20Component%20Object%20Reference) (OtherActor :type Actor%20Object%20Reference) (OtherComp :type Primitive%20Component%20Object%20Reference) (OtherBodyIndex :type Integer) (bFromSweep :type Boolean) (SweepResult :type Hit%20Result%20Structure%20%28by%20ref%29))
  (Variables|Default|SetBlendTime (Variables|Default|GetCustomBlendTime))
  (Game|Player|SetViewTargetwithBlend (Game|GetPlayerController 0) (stale EventBeginPlay _cameravariable) (Variables|Default|GetBlendTime) "VTBlend_EaseInOut" 3.0 false)
  (Variables|/Game/ThirdPersonBP/Blueprints/ThirdPersonGameMode.ThirdPersonGameMode_C|SetBP_SplineCamera (Variables|Default|GetGameMode) self))

(event Custom|Override%20Blend%20Cam
  (Variables|/Game/ThirdPersonBP/Blueprints/ThirdPersonGameMode.ThirdPersonGameMode_C|SetBP_SplineCamera (Variables|Default|GetGameMode) self)
  (Variables|Default|SetBlendTime (Variables|Default|GetCustomBlendTime))
  (Game|Player|SetViewTargetwithBlend (Game|GetPlayerController 0) (stale EventBeginPlay _cameravariable) (Variables|Default|GetBlendTime) "VTBlend_EaseInOut" 3.0 false)
  (Variables|/Game/ThirdPersonBP/Blueprints/ThirdPersonGameMode.ThirdPersonGameMode_C|SetBP_SplineCamera (Variables|Default|GetGameMode) self))

(event Custom|SetFirstCamera
  (bind _outactors (Actor|GetAllActorsOfClass "BP_SplineCamera_C"))
  (bind _output_get (Variables|Default|SetOtherSpline _outactors))
  (for _array_element _output_get
    (if (== _array_element self)
      (Variables|BP_SplineCamera_C|SetFirstCam%20?%20 _array_element true)
      (else
        (Variables|BP_SplineCamera_C|SetFirstCam%20?%20 _array_element false)))))

(event EventBeginPlay
  (bind _asthird_person_game_mode (Utilities|Casting|CastToThirdPersonGameMode (Game|GetGameMode)))
  (Variables|Default|SetGameMode _asthird_person_game_mode)
  (if (Variables|Default|GetFirstCam%20?%20)
    (bind _cameravariable (Variables|Default|GetCameraVariable)
      (:then
        (Variables|Default|SetBlendTime 0.0)
        (Game|Player|SetViewTargetwithBlend (Game|GetPlayerController 0) _cameravariable (Variables|Default|GetBlendTime) "VTBlend_EaseInOut" 3.0 false)
        (Variables|/Game/ThirdPersonBP/Blueprints/ThirdPersonGameMode.ThirdPersonGameMode_C|SetBP_SplineCamera (Variables|Default|GetGameMode) self))
      (:else))))

(event EventTick
  (params (DeltaSeconds :type Float%20%28single-precision%29))
  (bind _returnvalue (Game|Player|GetPlayerPawn 0))
  (bind _returnvalue_2 (CallFunction|CalculateLocation))
  (bind _spline (Variables|Default|GetSpline))
  (bind _cameravariable (Variables|Default|GetCameraVariable))
  (bind _returnvalue_3 (Transformation|GetActorLocation _returnvalue))
  (bind _returnvalue_4 (Spline|FindLocationClosesttoWorldLocation _spline _returnvalue_2 "World"))
  (bind _rootcomponent (Variables|/Script/Engine.Actor|GetRootComponent _cameravariable))
  (bind _returnvalue_5 (Transformation|GetWorldTransform _rootcomponent))
  (bind _returnvalue_6 (Math|Vector|Distance(Vector) _returnvalue_4 _returnvalue_3))
  ;[1 1 1] Movement of camera
  (Transformation|SetWorldLocationAndRotation _rootcomponent (Math|Interpolation|VInterpTo (.location _returnvalue_5) (+ _returnvalue_4 (Math|Vector|MakeVector (select (Variables|Default|GetAddOffset) (select (>= _returnvalue_6 7e+02) (Math|Float|MapRangeClamped _returnvalue_6 7e+02 1.2e+03 0.0 3.5e+02) (Math|Float|MapRangeClamped _returnvalue_6 7e+02 2e+02 0.0 -2.5e+02)) 0.0) 0.0 0.0)) DeltaSeconds 6.0) (select (Variables|Default|GetRotateCamera?%20) (Math|Interpolation|RInterpTo (.rotation _returnvalue_5) (Math|Rotator|FindLookatRotation (.location _returnvalue_5) _returnvalue_2) DeltaSeconds 3.0) "0, 0, 0") false false))

(fn ConstructionScript
  (bind _cameravariable (Variables|Default|GetCameraVariable)
    (:then
      (Transformation|SetWorldLocation (Variables|/Script/Engine.Actor|GetRootComponent _cameravariable) (Spline|GetLocationatTime (Variables|Default|GetSpline) (Variables|Default|GetDebugTime) "World" false) false false))
    (:else)))

(fn CalculateLocation
  (if (Variables|/Game/ThirdPersonBP/Blueprints/ThirdPersonGameMode.ThirdPersonGameMode_C|GetChoiceMode (Variables|Default|GetGameMode))
    (bind _returnvalue (Class|GameplayStatics|GetActorArrayAverageLocation (Variables|/Game/ThirdPersonBP/Blueprints/ThirdPersonGameMode.ThirdPersonGameMode_C|GetChoiceModeActors (Variables|Default|GetGameMode))))
    (return _returnvalue)
    (else
      (return (Transformation|GetActorLocation (Game|Player|GetPlayerPawn 0))))))